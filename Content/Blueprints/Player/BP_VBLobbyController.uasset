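; BP_VBLobbyController is the lobby player controller, handling the lobby screen, ready status and leaving.
; On BeginPlay it shows the cursor and uses an authority switch to create the host or client widget, with remote players also viewing a CameraActor.
; Ready toggles flip PlayerInfo and ask BP_VBLobbyGameMode to update player lists, while UpdatePlayerList forwards received info to the widget.
; Leaving destroys the session, then opens the main menu.
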(event Custom|CreateMenus
  (Networking|SwitchHasAuthority
    (:Authority
      (bind _returnvalue (UserInterface|CreateWidget "/Game/Blueprints/HUD/Menus/WBP_LobbyHostScreen.WBP_LobbyHostScreen_C"))
      (bind _output_get (Variables|Default|SetLobbyWidget _returnvalue))
      (UserInterface|Viewport|AddtoViewport _output_get 0))
    (:Remote
      (bind _returnvalue_2 (UserInterface|CreateWidget "/Game/Blueprints/HUD/Menus/WBP_LobbyClientScreen.WBP_LobbyClientScreen_C"))
      (bind _output_get_2 (Variables|Default|SetLobbyWidget _returnvalue_2))
      (UserInterface|Viewport|AddtoViewport _output_get_2 0)
      (bind _returnvalue_3 (Actor|GetActorOfClass "/Script/Engine.CameraActor"))
      (Game|Player|SetViewTargetwithBlend (Game|GetPlayerController 0) _returnvalue_3 0.0 "VTBlend_Linear" 0.0 false))))

(event Custom|UpdatePlayerList
  (params (PlayerInfo :type Array%20of%20Player%20Info%20Struct%20Structures))
  (bind _lobbywidget (Variables|Default|GetLobbyWidget))
  (bind _output_get (Variables|Default|SetConnectedPlayerInfo PlayerInfo))
  (Networking|SwitchHasAuthority
    (:Authority
      (bind _aswbp_lobby_host_screen (Utilities|Casting|CastToWBP_LobbyHostScreen _lobbywidget))
      (Default|UpdatePlayerList _aswbp_lobby_host_screen _output_get))
    (:Remote
      (bind _aswbp_lobby_client_screen (Utilities|Casting|CastToWBP_LobbyClientScreen _lobbywidget))
      (Default|UpdatePlayerList _aswbp_lobby_client_screen _output_get))))

(event Custom|LeaveLobby
  (bind _returnvalue (Game|GetPlayerController 0))
  (|DestroySession _returnvalue _returnvalue
    (:OnSuccess
      (Game|OpenLevel(byObjectReference) "/Game/OnlineMenuSubsystem/MainMenu.MainMenu"))))

(event Custom|SetReadyStatus
  (bind _playerinfo (Variables|Default|GetPlayerInfo))
  (Utilities|Struct|SetmembersinPlayerInfoStruct _playerinfo (not (Utilities|Struct|BreakPlayerInfoStruct _playerinfo)))
  (bind _asbp_vblobby_game_mode (Utilities|Casting|CastToBP_VBLobbyGameMode (Game|GetGameMode)))
  (Default|UpdatePlayerLists _asbp_vblobby_game_mode))

(event EventBeginPlay
  (CallFunction|CreateMenus)
  (Variables|Default|SetbShowMouseCursor true))

(fn ConstructionScript)