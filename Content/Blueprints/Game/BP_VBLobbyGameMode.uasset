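; Lobby game mode that tracks connected players with their names and ready states, and keeps each player's list in sync.
; On join, it records the controller and player info, marking the local host ready and others not ready.
; Joins, departures and list rebuilds push the info array to every lobby controller, with a short delay except on departures.
; A disconnect event makes all controllers leave the lobby.
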(event Custom|UpdatePlayerLists
  (bind _connectedplayerinfo (Variables|Default|GetConnectedPlayerInfo))
  ;[1 1 1] Update player lists
  (Utilities|Array|Clear (Variables|Default|GetConnectedPlayerInfo))
  (for _array_element (Variables|Default|GetConnectedPlayers)
    (if (Pawn|IsLocalController _array_element)
      (bind _output_get (Variables|/Game/Blueprints/Player/BP_VBLobbyController.BP_VBLobbyController_C|SetPlayerInfo _array_element (Variables|/Game/Blueprints/Player/BP_VBLobbyController.BP_VBLobbyController_C|GetPlayerInfo _array_element)))
      (Utilities|Array|Add _connectedplayerinfo _output_get)
      (else
        (Utilities|Array|Add _connectedplayerinfo (Variables|/Game/Blueprints/Player/BP_VBLobbyController.BP_VBLobbyController_C|GetPlayerInfo _array_element)))))
  (Utilities|FlowControl|Delay 0.4)
  (for _array_element_2 (Variables|Default|GetConnectedPlayers)
    (Default|UpdatePlayerList _array_element_2 (Variables|Default|GetConnectedPlayerInfo))))

(event Custom|DisconnectAllPlayers
  ;[1 1 1] Session destroyed
  (for _array_element (Variables|Default|GetConnectedPlayers)
    (Default|LeaveLobby _array_element)))

(event EventOnLogout
  (params (ExitingController :type Controller%20Object%20Reference))
  (bind _connectedplayers (Variables|Default|GetConnectedPlayers))
  (bind _connectedplayerinfo (Variables|Default|GetConnectedPlayerInfo))
  ;[1 1 1] Player left lobby
  (bind _aslobby_controller (Utilities|Casting|CastToBP_VBLobbyController ExitingController))
  (if (Utilities|Array|ContainsItem _connectedplayers _aslobby_controller)
    (Utilities|Array|RemoveItem _connectedplayers _aslobby_controller)
    (if (Utilities|Array|ContainsItem _connectedplayerinfo (Variables|/Game/Blueprints/Player/BP_VBLobbyController.BP_VBLobbyController_C|GetPlayerInfo _aslobby_controller))
      (Utilities|Array|RemoveItem _connectedplayerinfo (Variables|/Game/Blueprints/Player/BP_VBLobbyController.BP_VBLobbyController_C|GetPlayerInfo _aslobby_controller))
      (for _array_element (Variables|Default|GetConnectedPlayers)
        (Default|UpdatePlayerList _array_element (Variables|Default|GetConnectedPlayerInfo))))))

(event EventPostLogin
  (params (NewPlayer :type Player%20Controller%20Object%20Reference))
  (bind _connectedplayerinfo (Variables|Default|GetConnectedPlayerInfo))
  ;[1 1 1] Player joined lobby
  (bind _aslobby_controller (Utilities|Casting|CastToBP_VBLobbyController NewPlayer))
  (Utilities|Array|Add (Variables|Default|GetConnectedPlayers) _aslobby_controller)
  (if (Pawn|IsLocalController _aslobby_controller)
    (bind _output_get (Variables|/Game/Blueprints/Player/BP_VBLobbyController.BP_VBLobbyController_C|SetPlayerInfo _aslobby_controller (Utilities|Struct|MakePlayerInfoStruct (Utilities|Text|ToText(String) (PlayerState|GetPlayerName (Game|GetPlayerState 0))) true)))
    (Utilities|Array|Add _connectedplayerinfo _output_get)
    (else
      (bind _output_get_2 (Variables|/Game/Blueprints/Player/BP_VBLobbyController.BP_VBLobbyController_C|SetPlayerInfo _aslobby_controller (Utilities|Struct|MakePlayerInfoStruct (Utilities|Text|ToText(String) (PlayerState|GetPlayerName (Variables|/Script/Engine.Controller|GetPlayerState _aslobby_controller))) false)))
      (Utilities|Array|Add _connectedplayerinfo _output_get_2)))
  (Utilities|FlowControl|Delay 0.4)
  (for _array_element (Variables|Default|GetConnectedPlayers)
    (Default|UpdatePlayerList _array_element (Variables|Default|GetConnectedPlayerInfo))))

(fn ConstructionScript)