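; BP_VBGameMode is a game mode that handles match end and player disconnection for a multiplayer session.
; EndVBMatch loops over ConnectedControllers, calling LeaveLobby on each BP_VBPlayerController.
; Inside that same loop it calls DestroySession on player controller 0 each iteration, opening the MainMenu level on success.
; DisconnectAllPlayers runs the same LeaveLobby loop without destroying the session or changing level.
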(event Custom|DisconnectAllPlayers
  (for _array_element (Variables|Default|GetConnectedControllers)
    (bind _asbp_vbplayer_controller (Utilities|Casting|CastToBP_VBPlayerController _array_element))
    (Default|LeaveLobby _asbp_vbplayer_controller)))

(event EventEndVBMatch
  (for _array_element (Variables|Default|GetConnectedControllers)
    (bind _asbp_vbplayer_controller (Utilities|Casting|CastToBP_VBPlayerController _array_element))
    (Default|LeaveLobby _asbp_vbplayer_controller)
    (|DestroySession (Game|GetPlayerController 0)
      (:OnSuccess
        (Game|OpenLevel(byObjectReference) "/Game/OnlineMenuSubsystem/MainMenu.MainMenu")))))

(fn ConstructionScript)