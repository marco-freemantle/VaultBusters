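; Game instance for VaultBusters that handles LAN session hosting and joining, plus main menu music.
; Hosting creates an advanced session tagged with the game name and sized to the requested player count, then opens the lobby map as a listen server on success.
; Joining passes a given search result to the join node.
; Music plays as a 2D sound that persists across level transitions, with a guard against restarting while already playing.
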(event Custom|HostSession
  (params (NumberOfPlayers :type Integer))
  ;[1 1 1] Hosting and joining a session
  (bind _output_get (Variables|Default|SetNumber%20Of%20Players NumberOfPlayers))
  (|AdvancedSession (Utilities|Array|MakeArray (Class|AdvancedSessionsLibrary|MakeLiteralSessionPropertyString "GAMENAME" "VaultBusters")) (Game|GetPlayerController 0) _output_get 0 true true false true true true false false false true false true ; Make an advanced session with the extra session properties
    (:OnSuccess
      (Game|OpenLevel(byObjectReference) "/Game/Maps/LobbyMap.LobbyMap" true "listen"))))

(event Custom|JoinSession
  (params (Session :type Blueprint%20Session%20Result%20Structure))
  ;[1 1 1] Hosting and joining a session
  (|JoinSession (Game|GetPlayerController 0) Session))

(event Custom|PlayMusic
  ;[1 1 1] Music
  (Utilities|IsValid (Variables|Default|GetMusic)
    (:Is%20Valid
      (if (not (Audio|Components|Audio|IsPlaying (Variables|Default|GetMusic)))
        (bind _returnvalue (Audio|SpawnSound2D "/Game/Assets/Sounds/Music/Music_MainMenu.Music_MainMenu" 1.0 1.0 0.0 0 true :!label _label))
        (Variables|Default|SetMusic _returnvalue)))
    (:Is%20Not%20Valid
      (goto _label))))

(event Custom|StopMusic
  ;[1 1 1] Music
  (Audio|Components|Audio|Stop (Variables|Default|GetMusic)))